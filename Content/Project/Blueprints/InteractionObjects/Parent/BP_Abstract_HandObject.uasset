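; Abstract parent Blueprint for objects that can be grabbed and released, named as hand objects.
; Grab snaps location and rotation to the supplied attach point, keeps relative scale, and turns off RootHandObject physics and Cube collision.
; Release detaches the actor in world space, re-enables physics and restores Cube collision as query-only.
; Both functions return false, and the event graph and construction script are empty.
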(event EventBeginPlay)

(event Collision|EventActorBeginOverlap
  (params (OtherActor :type Actor%20Object%20Reference)))

(event EventTick
  (params (DeltaSeconds :type Float%20%28single-precision%29)))

(fn ConstructionScript)

(fn Grab
  (params (Attach%20Point :type Scene%20Component%20Object%20Reference))
  (Transformation|AttachComponentToComponent Attach%20Point "None" "SnapToTarget" "SnapToTarget" "KeepRelative" true)
  (Physics|SetSimulatePhysics (Variables|Default|GetRoot%20Hand%20Object) false)
  (Collision|SetCollisionEnabled (Variables|Default|GetCube) "NoCollision")
  (return false))

(fn Release
  (Transformation|DetachFromActor "KeepWorld" "KeepWorld" "KeepWorld")
  (Physics|SetSimulatePhysics (Variables|Default|GetRoot%20Hand%20Object) true)
  (Collision|SetCollisionEnabled (Variables|Default|GetCube) "QueryOnly")
  (return false))