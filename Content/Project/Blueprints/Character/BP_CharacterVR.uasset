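; BP_CharacterVR is a VR character that owns two motion controller hands for grabbing.
; On BeginPlay it sets floor-level tracking, spawns a left and a right BP_VR_MotionController attached to the camera root, and applies a position-only HMD base offset.
; Grab and Release forward to the left or right controller based on an IsRightHand flag.
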(event EventBeginPlay
  (CallFunction|ConfigureOptionsforVR))

(fn ConstructionScript)

(fn ConfigureOptionsforVR
  (Class|HeadMountedDisplayFunctionLibrary|SetTrackingOrigin "Floor")
  (bind _returnvalue (Game|SpawnActorfromClass "/Game/Project/Blueprints/Character/BP_VR_MotionController.BP_VR_MotionController_C" (Math|Transform|MakeTransform "0, 0, 0") "AlwaysSpawn" self "Left" 0))
  (bind _output_get (Variables|Default|SetLeft%20Controller _returnvalue))
  (Transformation|AttachComponentToComponent _output_get (Variables|Default|GetCamera%20Root%20Component) "None" "SnapToTarget" "SnapToTarget" "KeepRelative" true)
  (bind _returnvalue_2 (Game|SpawnActorfromClass "/Game/Project/Blueprints/Character/BP_VR_MotionController.BP_VR_MotionController_C" (Math|Transform|MakeTransform "0, 0, 0") "AlwaysSpawn" self "Right" 0))
  (bind _output_get_2 (Variables|Default|SetRight%20Controller _returnvalue_2))
  (Transformation|AttachComponentToComponent _output_get_2 (Variables|Default|GetCamera%20Root%20Component) "None" "SnapToTarget" "SnapToTarget" "KeepRelative" true)
  (Class|OculusFunctionLibrary|SetBaseRotationandBaseOffsetinMeters "0, 0, 0" "0, 0,0.500000" "Position"))

(fn Grab
  (params (isRightHand :type Boolean))
  (if isRightHand
    (Default|Grab (Variables|Default|GetRight%20Controller))
    (else
      (Default|Grab (Variables|Default|GetLeft%20Controller)))))

(fn Release
  (params (isRightHand :type Boolean))
  (if isRightHand
    (Default|Release (Variables|Default|GetRight%20Controller))
    (else
      (Default|Release (Variables|Default|GetLeft%20Controller)))))