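; VR hand actor that grabs and releases hand objects, with its motion source set from HandType at construction.
; Grab takes only the first actor overlapping HandCollision and checks its Mass against the LevelOfPower on the player controller cached at BeginPlay.
; The two lower levels set maximum masses, while level 2 accepts only objects above a minimum.
; Accepted objects receive GrabMessage with AttachPoint, and Release sends ReleaseMessage.
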(event EventBeginPlay
  (bind _asbp_vr_player_controller (Utilities|Casting|CastToBP_VR_PlayerController (Game|GetPlayerController 0)))
  (Variables|Default|SetPlayer%20Controller _asbp_vr_player_controller))

(event Collision|EventActorBeginOverlap
  (params (OtherActor :type Actor%20Object%20Reference)))

(event EventTick
  (params (DeltaSeconds :type Float%20%28single-precision%29)))

(fn ConstructionScript
  (Variables|/Script/HeadMountedDisplay.MotionControllerComponent|SetMotionSource (Variables|Default|GetMotionController) (Variables|Default|GetHandType)))

(fn Grab
  (bind _asbp_abstract_hand_object (Utilities|Casting|CastToBP_Abstract_HandObject (Utilities|Array|Get(acopy) (Collision|GetOverlappingActors (Variables|Default|GetHandCollision) 0 :!class /Script/Engine.PrimitiveComponent))))
  (bind _output_get (Variables|Default|SetGrabbed%20Actor _asbp_abstract_hand_object))
  (LocalVariables|SetCurrent%20Mass (Variables|/Game/Project/Blueprints/InteractionObjects/Parent/BP_Abstract_HandObject.BP_Abstract_HandObject_C|GetMass _output_get))
  (switch int (Variables|/Game/Project/Blueprints/Character/BP_VR_PlayerController.BP_VR_PlayerController_C|GetLevel%20of%20Power (Variables|Default|GetPlayer%20Controller))
    (:0
      (if (<= (LocalVariables|GetCurrent%20Mass) 5e+01)
        (Class|INTHandObjects|Grab(Message) (Variables|Default|GetGrabbed%20Actor) (Variables|Default|GetAttachPoint) :!label _label)
        (else
          (Variables|Default|SetGrabbed%20Actor 0 :!label _label_2))))
    (:1
      (if (<= (LocalVariables|GetCurrent%20Mass) 1e+02)
        (goto _label)
        (else
          (goto _label_2))))
    (:2
      (if (> (LocalVariables|GetCurrent%20Mass) 5e+01)
        (goto _label)
        (else
          (goto _label_2))))))

(fn Release
  (bind _grabbed_actor (Variables|Default|GetGrabbed%20Actor)
    (:then
      (Class|INTHandObjects|Release(Message) _grabbed_actor)
      (Variables|Default|SetGrabbed%20Actor 0))
    (:else)))