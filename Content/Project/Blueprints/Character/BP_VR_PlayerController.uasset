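; VR player controller that forwards left and right hand grab/release input to BP_CharacterVR and steps a three-level "power" setting up or down.
; Increase and decrease inputs set a target value and play or reverse the Increase timeline, which stops on reaching that target.
; The timeline's output drives the Z component of the tracking base offset, shifting the player's VR view vertically between levels.
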(event Custom|Set%20New%20Time%20in%20Power%20Timeline
  ;[1 1 1] Change Power by Trigger
  (bind _current_power (Timeline|Increase SetNewTime)
    (:Update
      (Class|OculusFunctionLibrary|SetBaseRotationandBaseOffsetinMeters "0, 0, 0" (Math|Vector|MakeVector 0.0 0.0 _current_power) "Position")
      (if (Math|Float|NearlyEqual(Float) (Variables|Default|GetPower%20Value) _current_power 0.01)
        (Timeline|Increase Stop)))))

(event EventBeginPlay
  (bind _asbp_character_vr (Utilities|Casting|CastToBP_CharacterVR (Game|GetPlayerCharacter 0)))
  (Variables|Default|SetPlayer%20Character _asbp_character_vr)
  (CallFunction|SetNewTimeinPowerTimeline))

(event Input|ActionEvents|InputActionRHandGrabRelease
  (params (Key :type Key%20Structure :default "None"))
  ;[1 1 1] Grab Objects
  (:Pressed
    (Default|Grab (Variables|Default|GetPlayer%20Character) true))
  (:Released
    (Default|Release (Variables|Default|GetPlayer%20Character) true)))

(event Input|ActionEvents|InputActionLHandGrabRelease
  (params (Key :type Key%20Structure :default "None"))
  ;[1 1 1] Grab Objects
  (:Pressed
    (Default|Grab (Variables|Default|GetPlayer%20Character) false))
  (:Released
    (Default|Release (Variables|Default|GetPlayer%20Character) false)))

(event Input|ActionEvents|InputActionIncreasePower
  (params (Key :type Key%20Structure :default "None"))
  ;[1 1 1] Change Power by Trigger
  (:Pressed
    (switch int (Variables|Default|GetLevel%20of%20Power)
      (:0
        (Variables|Default|SetPower%20Value 0.5)
        (Variables|Default|SetLevel%20of%20Power 1)
        (bind _current_power (Timeline|Increase Play)
          (:Update
            (Class|OculusFunctionLibrary|SetBaseRotationandBaseOffsetinMeters "0, 0, 0" (Math|Vector|MakeVector 0.0 0.0 _current_power) "Position")
            (if (Math|Float|NearlyEqual(Float) (Variables|Default|GetPower%20Value) _current_power 0.01)
              (Timeline|Increase Stop)))))
      (:1
        (Variables|Default|SetPower%20Value 0.0)
        (Variables|Default|SetLevel%20of%20Power 2)
        (Timeline|Increase Play)))))

(event Input|ActionEvents|InputActionDecreasePower
  (params (Key :type Key%20Structure :default "None"))
  ;[1 1 1] Change Power by Trigger
  (:Pressed
    (switch int (Variables|Default|GetLevel%20of%20Power)
      (:1
        (Variables|Default|SetPower%20Value 1.0)
        (Variables|Default|SetLevel%20of%20Power 0)
        (bind _current_power (Timeline|Increase Reverse)
          (:Update
            (Class|OculusFunctionLibrary|SetBaseRotationandBaseOffsetinMeters "0, 0, 0" (Math|Vector|MakeVector 0.0 0.0 _current_power) "Position")
            (if (Math|Float|NearlyEqual(Float) (Variables|Default|GetPower%20Value) _current_power 0.01)
              (Timeline|Increase Stop)))))
      (:2
        (Variables|Default|SetPower%20Value 0.5)
        (Variables|Default|SetLevel%20of%20Power 1)
        (Timeline|Increase Reverse)))))

(fn ConstructionScript)